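; Actor component for a combo system that records incoming input actions in a buffer, with no live combo matching yet.
; Each ComboReceived event appends to the buffer, restarts a timer that clears it after a few idle seconds, and prints the sequence for debugging.
; An unconnected test sketches combo lookup by filtering data table rows on weapon type and searching their inputs.
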(event `Reset Buffer`
  (set `self.InputBuffer` (`|MakeArray`))
  (`KismetSystemLibrary.PrintString` "Reset Input Buffer"))

(event `ComboEvent Received`
  (params (`Input Action` :type "InputAction Object Reference"))
  (bind _inputbuffer (`self.InputBuffer`))
  (`KismetArrayLibrary.Array_Add` _inputbuffer `Input Action`)
  (`KismetSystemLibrary.K2_SetTimerDelegate` (delegate `Reset Buffer`) 5.0)
  (set `self.Inputs` "")
  (for _array_element _inputbuffer
    (set `self.Inputs` (`KismetStringLibrary.Concat_StrStr` (`self.Inputs`) ">" (`KismetSystemLibrary.GetDisplayName` _array_element))))
  (`KismetSystemLibrary.PrintString` (`KismetStringLibrary.Concat_StrStr` (`KismetStringLibrary.Conv_IntToString` (`KismetArrayLibrary.Array_Length` _inputbuffer)) " - " (`self.Inputs`)) true true (struct :`G` 0.66 :`B` 1.0 :`A` 1.0) 5.0))