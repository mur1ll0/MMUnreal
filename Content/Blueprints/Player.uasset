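; Player character Blueprint that handles Enhanced Input movement, camera look, jumping and forwarding left/right clicks to ACComboSystem.
; Movement follows camera yaw and turns on controller-desired rotation only while moving.
; Tick computes the control-to-actor rotation delta as TurnInPlaceRotation, and BeginPlay caches the ABP_Player anim instance.
; Also holds an unconnected camera-relative dodge, an angle-normalizing helper and a tap/hold input macro.
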(event `self.ReceiveBeginPlay`
  ;[1 1 1] Mapeando contexto
  (bind _asbp_player_controller (cast `/Game/Blueprints/BP_PlayerController` (`self.GetController`)))
  (bind _returnvalue (pcsubsystem `EnhancedInputLocalPlayerSubsystem` _asbp_player_controller))
  (`/Engine/EditorBlueprintResources/StandardMacros.IsValid` _returnvalue
    (:`Is Valid`
      (`EnhancedInputSubsystemInterface.AddMappingContext` _returnvalue "/Game/Controls/IMC_Controls.IMC_Controls" 0 (struct))
      (bind _asabp_player (cast `/Game/Blueprints/ABP_Player` (`SkeletalMeshComponent.GetAnimInstance` (`self.Mesh`))))
      (set `self.As ABP Player` _asabp_player))))

(event `EnhancedInput|/Game/Controls/Inputs/IA_Move`
  (params (ActionValue :type "Vector2D Structure") (ElapsedSeconds :type "Float (double-precision)") (TriggeredSeconds :type "Float (double-precision)") (InputAction :type "InputAction Object Reference" :default "/Game/Controls/Inputs/IA_Move.IA_Move"))
  (bind (_returnvalue_roll _returnvalue_pitch _returnvalue_yaw) (`KismetMathLibrary.BreakRotator` (`self.GetControlRotation`)))
  ;[1 1 1] Movimentos WASD
  (:`Triggered`
    (set `self.ControllerDirection` (`KismetMathLibrary.MakeVector` ActionValue_Y ActionValue_X))
    (`self.AddMovementInput` (`KismetMathLibrary.GetRightVector` (`KismetMathLibrary.MakeRotator` _returnvalue_roll 0.0 _returnvalue_yaw)) ActionValue_X)
    (`self.AddMovementInput` (`KismetMathLibrary.GetForwardVector` (`KismetMathLibrary.MakeRotator` 0.0 0.0 _returnvalue_yaw)) ActionValue_Y)
    ;;[1 0.165 0.2148] Ativar Char Rotation quando em movimento
    (`self.SetCharRotationControl` true)
    ;;[0.1413 0 1] Variáveis de controle
    (set `self.ControlMoving` true))
  (:`Completed`
    (`self.SetCharRotationControl` false)
    (set `self.ControlMoving` false)))

(event `EnhancedInput|/Game/Controls/Inputs/IA_Look`
  (params (ActionValue :type "Vector2D Structure") (ElapsedSeconds :type "Float (double-precision)") (TriggeredSeconds :type "Float (double-precision)") (InputAction :type "InputAction Object Reference" :default "/Game/Controls/Inputs/IA_Look.IA_Look"))
  ;[1 1 1] Movimento da camera X / Y
  (:`Triggered`
    (`self.AddControllerYawInput` ActionValue_X)
    (`self.AddControllerPitchInput` ActionValue_Y)
    ;;[0.1413 0 1] Variáveis de controle
    (set `self.MouseMoving` true))
  (:`Completed`
    (set `self.MouseMoving` false)))

(event `EnhancedInput|/Game/Controls/Inputs/IA_Jump`
  (params (ActionValue :type Boolean) (ElapsedSeconds :type "Float (double-precision)") (TriggeredSeconds :type "Float (double-precision)") (InputAction :type "InputAction Object Reference" :default "/Game/Controls/Inputs/IA_Jump.IA_Jump"))
  ;[1 1 1] Pular
  (:`Triggered`
    (`self.Jump`))
  (:`Completed`
    (`self.StopJumping`)))

(event `self.ReceiveTick`
  (params (DeltaSeconds :type "Float (single-precision)"))
  ;[1 1 1] Calcular ângulo entre personagem e a mira
  (set `self.TurnInPlaceRotation` (`KismetMathLibrary.NormalizedDeltaRotator` (`self.GetControlRotation`) (`self.K2_GetActorRotation`))))

(event `EnhancedInput|/Game/Controls/Inputs/IA_LeftClick`
  (params (ActionValue :type Boolean) (ElapsedSeconds :type "Float (double-precision)") (TriggeredSeconds :type "Float (double-precision)") (InputAction :type "InputAction Object Reference" :default "/Game/Controls/Inputs/IA_LeftClick.IA_LeftClick"))
  (:`Started`
    (`/Game/Components/ComboSystem/AC_ComboSystem.ComboEvent Received` (`self.AC_ComboSystem`) InputAction)))

(event `EnhancedInput|/Game/Controls/Inputs/IA_RightClick`
  (params (ActionValue :type Boolean) (ElapsedSeconds :type "Float (double-precision)") (TriggeredSeconds :type "Float (double-precision)") (InputAction :type "InputAction Object Reference" :default "/Game/Controls/Inputs/IA_RightClick.IA_RightClick"))
  (:`Started`
    (`/Game/Components/ComboSystem/AC_ComboSystem.ComboEvent Received` (`self.AC_ComboSystem`) InputAction)))

(fn `GetControllerDirectionRotation`
  (params (Direction :type "Vector Structure"))
  (returns (Rotation :type "Rotator Structure"))
  (bind _returnvalue (`CharacterMovementComponent.GetLastUpdateLocation` (`self.CharacterMovement`)))
  (return (`KismetMathLibrary.FindLookAtRotation` _returnvalue (+ _returnvalue (`KismetMathLibrary.Normal` (`KismetMathLibrary.GreaterGreater_VectorRotator` Direction (`KismetMathLibrary.MakeRotator` 0.0 0.0 (.yaw (`self.GetControlRotation`)))))))))

(fn `NormalizeAngle`
  (params (Angle :type "Float (double-precision)"))
  (returns (`Normalized Angle` :type "Float (double-precision)"))
  (locals (NewAngle :type "Float (double-precision)"))
  (if (> Angle 180.0)
    (set `local.NewAngle` (- Angle 360.0))
    (elif (< Angle -180.0)
      (set `local.NewAngle` (+ Angle 360.0))
      (else
        (set `local.NewAngle` Angle))))
  (return (`local.NewAngle`)))

(fn `SetCharRotationControl`
  (params (CharRotation :type Boolean))
  (bind _charactermovement (`self.CharacterMovement`))
  (if CharRotation
    (set `CharacterMovementComponent.bUseControllerDesiredRotation` true _charactermovement)
    (set `CharacterMovementComponent.bOrientRotationToMovement` false _charactermovement)
    (set `self.bUseControllerRotationYaw` false)
    (else
      (set `CharacterMovementComponent.bUseControllerDesiredRotation` false _charactermovement)
      (set `CharacterMovementComponent.bOrientRotationToMovement` false _charactermovement)
      (set `self.bUseControllerRotationYaw` false))))

(fn `UserConstructionScript`)